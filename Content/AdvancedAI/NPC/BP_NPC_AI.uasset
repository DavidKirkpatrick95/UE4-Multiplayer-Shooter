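; BP_NPC_AI is the AI controller for NPCs, starting their BT_NPC behavior tree on BeginPlay.
; It then casts the controlled pawn to BP_NPC_Health and stores it, stopping if the cast fails.
; It seeds the blackboard from that pawn's patrol path with looping and wait time, plus an initial forward direction for patrol movement.
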(event EventBeginPlay
  (AI|RunBehaviorTree "/Game/AdvancedAI/NPC/BT_NPC.BT_NPC")
  (bind _asbp_npc_health (Utilities|Casting|CastToBP_NPC_Health (Pawn|GetControlledPawn)))
  (bind _output_get (Variables|Default|SetMyPawn _asbp_npc_health))
  (AI|Components|Blackboard|SetValueasBool (AI|GetBlackboard 0) (Utilities|Name|MakeLiteralName "PathLooping") (Variables|/Game/AdvancedAI/NPC/PatrolPath.PatrolPath_C|GetIsLooping (Variables|/Game/AdvancedAI/NPC/BP_NPC_Health.BP_NPC_Health_C|GetPatrolPath _output_get)))
  (Class|BlackboardComponent|SetValueasInt (AI|GetBlackboard 0) (Utilities|Name|MakeLiteralName "Direction") 1)
  (AI|Components|Blackboard|SetValueasFloat (AI|GetBlackboard 0) (Utilities|Name|MakeLiteralName "WaitTime") (Variables|/Game/AdvancedAI/NPC/PatrolPath.PatrolPath_C|GetWaitTime (Variables|/Game/AdvancedAI/NPC/BP_NPC_Health.BP_NPC_Health_C|GetPatrolPath (Variables|Default|GetMyPawn)))))

(event EventTick
  (params (DeltaSeconds :type Float%20%28single-precision%29)))

(fn ConstructionScript)