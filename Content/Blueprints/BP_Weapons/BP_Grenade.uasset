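; BP_Grenade is a timed grenade actor that detonates shortly after BeginPlay.
; After a fixed delay, its Explode event spawns an explosion particle, then radial damage is applied at the actor's location, credited to the instigator's controller and blockable on the WorldStatic channel.
; The actor then destroys itself and draws a brief debug sphere showing the damage radius.
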(event Custom|Explode
  (Effects|SpawnEmitteratLocation "/Game/WeaponEffects/Explosion/P_Explosion.P_Explosion" (Transformation|GetActorLocation)))

(event EventBeginPlay
  (bind _returnvalue (Transformation|GetActorLocation))
  (Utilities|FlowControl|Delay 1.0)
  (CallFunction|Explode)
  (Game|Damage|ApplyRadialDamage 4e+02 _returnvalue (Variables|Default|GetDamageRadius) "/Script/Engine.DamageType" 0 self (Game|GetInstigatorController) false "ECC_WorldStatic")
  (Actor|DestroyActor)
  (Rendering|Debug|DrawDebugSphere _returnvalue (Variables|Default|GetDamageRadius) 12 "(R=1.000000,G=0.010197,B=0.030093,A=1.000000)" 1.0 1.0))

(fn ConstructionScript)