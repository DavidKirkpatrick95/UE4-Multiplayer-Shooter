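; Explosive barrel actor that blows up once when its health is depleted.
; The SHealth component's OnHealthChanged event calls Explode through a DoOnce when health reaches zero or below.
; Explode swaps the mesh to an exploded material, launches it upward with an impulse, spawns an explosion particle effect and fires the RadialForce impulse.
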(event OnHealthChanged(SHealth)
  (params (HealthComp :type S%20Health%20Component%20Object%20Reference) (Health :type Float%20%28single-precision%29) (HealthDelta :type Float%20%28single-precision%29) (DamageType :type Damage%20Type%20Object%20Reference) (InstigatedBy :type Controller%20Object%20Reference) (DamageCauser :type Actor%20Object%20Reference))
  (if (<= Health 0.0)
    (Utilities|FlowControl|DoOnce false
      (:Completed
        (CallFunction|Explode)))))

(event EventBeginPlay)

(event Collision|EventActorBeginOverlap
  (params (OtherActor :type Actor%20Object%20Reference)))

(event EventTick
  (params (DeltaSeconds :type Float%20%28single-precision%29)))

(fn ConstructionScript)

(fn Explode
  (Rendering|Material|SetMaterial (Variables|Default|GetBarrelMesh) 0 "/Game/BarrelResources/Challenges/ExplosiveBarrel/M_ExplosiveBarrelExploded.M_ExplosiveBarrelExploded")
  (Physics|AddImpulse (Variables|Default|GetBarrelMesh) "0, 0,62500.000000" "None" false)
  (Effects|SpawnEmitteratLocation "/Game/WeaponEffects/Explosion/P_Explosion.P_Explosion" (Transformation|GetWorldLocation (Variables|Default|GetBarrelMesh)))
  (Class|RadialForceComponent|FireImpulse (Variables|Default|GetRadialForce)))